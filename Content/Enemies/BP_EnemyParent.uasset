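; BP_EnemyParent is the base enemy for a tower defense mode, walking to the goal actor as soon as play begins.
; GoToGoal waits briefly, applies EnemySpeed to the movement component, then runs AI MoveTo toward the first GoalOfEnemies found in the level.
; On arrival the enemy destroys itself and decrements TotalOfEnemies on GM_TowerDefense.
; A failed move calls GoToGoal again to retry.
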(event Custom|GoToGoal
  ;[0.375 0.375 0.375 0.432] Bouge les enemies vers le GOAL
  (Utilities|FlowControl|Delay 0.2)
  (Variables|/Script/Engine.CharacterMovementComponent|SetMaxWalkSpeed (Variables|Character|GetCharacterMovement) (Variables|Default|GetEnemySpeed))
  (bind _outactors (Actor|GetAllActorsOfClass "/Game/LevelElement/GoalNSpawn/GoalOfEnemies.GoalOfEnemies_C"))
  (AI|AIMoveTo self "0, 0, 0" (Utilities|Array|Get(acopy) _outactors) 2e+02 false
    (:OnSuccess
      (Development|PrintString "Enemy Success")
      (Actor|DestroyActor)
      (bind _asgm_tower_defense (Utilities|Casting|CastToGM_TowerDefense (Game|GetGameMode)))
      (bind _output_get (Variables|Default|SetGameMode _asgm_tower_defense))
      (Variables|/Game/TD_Blueprints/GM_TowerDefense.GM_TowerDefense_C|SetTotalOfEnemies _output_get (- (Variables|/Game/TD_Blueprints/GM_TowerDefense.GM_TowerDefense_C|GetTotalOfEnemies _output_get) 1)))
    (:OnFail
      (CallFunction|GotoGoal))))

(event EventBeginPlay
  ;[0.375 0.375 0.375 0.432] Bouge les enemies vers le GOAL
  (CallFunction|GotoGoal))

(fn ConstructionScript)