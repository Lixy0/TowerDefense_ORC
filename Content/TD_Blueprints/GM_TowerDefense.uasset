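; Tower defense game mode that runs data-driven waves of golem enemies.
; PopulateMap reads the wave's data table row into a map of enemy class to remaining count.
; A looping timer calls ChooseEnemy, which randomly draws and decrements a class, or starts the next wave once none remain queued or alive.
; The random spawn-point SpawnEnemy call is disconnected, so chosen enemies never spawn.
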(event Custom|ActivateSpawner
  ;[0.3229 0.3229 0.3229 0.474] Gestion des spawn point de façon hasardeuse
  (if (> (Variables|Default|GetNumberOfEnemies) 0)
    (bind _enemychosen (CallFunction|ChooseEnemy))
    (else
      ;[0.1383 0.1315 0.25 0.573] Wave d'ennemies
      (bind _outactors (Actor|GetAllActorsOfClass "/Game/Enemies/BP_EnemyParent.BP_EnemyParent_C"))
      (if (<= (Utilities|Array|Length _outactors) 0)
        (bind _result (Math|Integer|IncrementInt (Variables|Default|GetWaveNumber))
          (:%20%20
            (CallFunction|PopulateMap _result)))))))

(event EventBeginPlay
  ;[0.3229 0.3229 0.3229 0.474] Gestion des spawn point de façon hasardeuse
  (bind _outactors (Actor|GetAllActorsOfClass "/Game/LevelElement/GoalNSpawn/SpawnPoint.SpawnPoint_C"))
  (Variables|Default|SetListOfSpawnPoint _outactors)
  (Utilities|Time|SetTimerbyEvent (delegate Custom|ActivateSpawner) 2.0 true)
  (CallFunction|PopulateMap (Variables|Default|GetWaveNumber)))

(fn ConstructionScript)

(fn PopulateMap
  (params (WaveNumber :type Integer))
  (bind _returnvalue (Utilities|GetDataTableRow "/Game/Enemies/WaveDetailsDataTable.WaveDetailsDataTable" (Utilities|String|StringToName (Utilities|String|ToString(Integer) WaveNumber)))
    (:then
      (Variables|Default|SetTotalOfEnemies (+ (.golem_small _returnvalue) (.golem_large _returnvalue) (.golem_xl _returnvalue)))
      (bind _output_get (Variables|Default|SetEnemyList (Utilities|Map|MakeMap "/Game/Enemies/BP_EnemyGolemSmall.BP_EnemyGolemSmall_C" (.golem_small _returnvalue) "/Game/Enemies/BP_EnemyGolemLarge.BP_EnemyGolemLarge_C" (.golem_large _returnvalue) "/Game/Enemies/BP_EnemyGolemXL.BP_EnemyGolemXL_C" (.golem_xl _returnvalue))))
      (bind _values (Utilities|Map|Values _output_get))
      (for _array_element _values
        (Variables|Default|SetNumberOfEnemies (+ _array_element (Variables|Default|GetNumberOfEnemies)))))))

(fn ChooseEnemy
  (bind _keys (Utilities|Map|Keys (Variables|Default|GetEnemyList) :!label _label))
  (bind _output_get (Variables|Default|SetChosenEnemy (Utilities|Array|Get(acopy) _keys (Math|Random|RandomInteger (Utilities|Array|Length _keys)))))
  (Variables|Default|SetEnemyNumber (.Value (Utilities|Map|Find (Variables|Default|GetEnemyList) _output_get)))
  (if (> (.Value (Utilities|Map|Find (Variables|Default|GetEnemyList) _output_get)) 0)
    (Utilities|Map|Add (Variables|Default|GetEnemyList) (Variables|Default|GetChosenEnemy) (- (Variables|Default|GetEnemyNumber) 1))
    (Variables|Default|SetNumberOfEnemies (- (Variables|Default|GetNumberOfEnemies) 1))
    (return (Variables|Default|GetChosenEnemy))
    (else
      (goto _label))))